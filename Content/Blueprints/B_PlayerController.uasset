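; Player controller that switches the player between the menu camera, console and highscore pawns.
; Each switch runs from an input action or a matching Possess event, finding the first actor of that class in the level.
; It eases the view target over to that actor across SwitchSpeed seconds, waits out the blend, then possesses it, printing a debug label.
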(event `PossessMenu`
  (bind _switchspeed (`self.SwitchSpeed`))
  (`KismetSystemLibrary.PrintString` "Camera" :!label _label)
  (bind _outactors (`GameplayStatics.GetAllActorsOfClass` "/Game/Blueprints/BP_Camera.BP_Camera_C"))
  (bind _output (`|GetArrayItem` _outactors))
  (`self.SetViewTargetWithBlend` _output _switchspeed "VTBlend_EaseInOut" 3.0)
  (`KismetSystemLibrary.Delay` _switchspeed)
  (`self.Possess` _output))

(event `InputAction|MenuCamera`
  (params (Key :type "Key Structure"))
  (:`Pressed`
    (goto _label)))

(event `PossessConsole`
  (bind _switchspeed (`self.SwitchSpeed`))
  (`KismetSystemLibrary.PrintString` "Console" :!label _label_2)
  (bind _outactors (`GameplayStatics.GetAllActorsOfClass` "/Game/Blueprints/BP_Console_Pawn.BP_Console_Pawn_C"))
  (bind _output (`|GetArrayItem` _outactors))
  (`self.SetViewTargetWithBlend` _output _switchspeed "VTBlend_EaseInOut" 3.0)
  (`KismetSystemLibrary.Delay` _switchspeed)
  (`self.Possess` _output))

(event `InputAction|Console`
  (params (Key :type "Key Structure"))
  (:`Pressed`
    (goto _label_2)))

(event `PossessHighscore`
  (bind _switchspeed (`self.SwitchSpeed`))
  (`KismetSystemLibrary.PrintString` "Highscore" :!label _label_3)
  (bind _outactors (`GameplayStatics.GetAllActorsOfClass` "/Game/Blueprints/BP_Highscore.BP_Highscore_C"))
  (bind _output (`|GetArrayItem` _outactors))
  (`self.SetViewTargetWithBlend` _output _switchspeed "VTBlend_EaseInOut" 3.0)
  (`KismetSystemLibrary.Delay` _switchspeed)
  (`self.Possess` _output))

(event `InputAction|Highscore`
  (params (Key :type "Key Structure"))
  (:`Pressed`
    (goto _label_3)))

(fn `UserConstructionScript`)