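; Game mode for a handheld-console-style egg-catching game, running scoring, fails, difficulty and game over for two game variants.
; A delay-driven BeginPlay loop spawns eggs on non-repeating tracks, tightening intervals as play progresses, with score milestones easing pace and fails.
; EggDestiny compares track to wolf direction to score or fail, with rabbit presence halving penalties.
; BP_Console_Pawn handles rendering and sound; game over appends results to a highscore save.
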(event `self.ReceiveBeginPlay`
  ;[1 1 1] Game Logic
  (if (`self.isGameStarted`) :!label _label
    (if (not (`self.isRabbitTimer`))
      (set `self.isRabbitTimer` true)
      (`KismetSystemLibrary.K2_SetTimer` (`GameplayStatics.GetPlayerPawn` 0) "RabbitToggle" (`KismetMathLibrary.RandomFloatInRange` 5.0 10.0)))
    (if (`self.isFell`)
      (`KismetSystemLibrary.Delay` 3.0)
      (set `self.isFell` false)
      (else
        (`self.UpdateIntervals`)))
    (`self.Spawn`)
    (`KismetSystemLibrary.Delay` (`self.EggSpawnInterval`))
    (goto _label)
    (else
      (if (`self.isReset`)
        (`KismetSystemLibrary.Delay` (`self.EggTick`))
        (`self.ResetGameData`)
        (set `self.isReset` false)
        (set `self.isGameStarted` true))
      (`KismetSystemLibrary.Delay` 0.05)
      (goto _label))))

(event `SelectGameMode`
  (params (GameMode :type Boolean))
  ;[1 1 1] Select Game Mode
  (set `self.isGameStarted` false)
  (set `self.GameMode` GameMode)
  (set `self.isReset` true)
  (`/Game/Blueprints/BP_Console_Pawn.EggsTurnOff` (cast `/Game/Blueprints/BP_Console_Pawn` (`GameplayStatics.GetPlayerPawn` 0) :!pure true))
  (set `self.EggTick` 1.0)
  (set `self.EggSpawnInterval` 2.0)
  (`GameplayStatics.SetGlobalTimeDilation` 1.0))

(event `ResetGameData`
  (bind _asbp_console_pawn (cast `/Game/Blueprints/BP_Console_Pawn` (`GameplayStatics.GetPlayerPawn` 0) :!pure true))
  ;[1 1 1] Reset Game Data
  (set `self.isFell` false)
  (set `self.isAdjustedForGameB` false)
  (set `self.LastUsedTrack` -1)
  (set `self.Fails` 0)
  (set `self.Score` 0)
  (`/Game/Blueprints/BP_Console_Pawn.ScoreRender` _asbp_console_pawn)
  (`/Game/Blueprints/BP_Console_Pawn.FailRender` _asbp_console_pawn))

(event `EggDestiny`
  (params (Track :type Integer))
  ;[1 1 1] Egg Destiny
  (if (`KismetMathLibrary.BooleanNOR` (`self.isFell`) (`self.isReset`))
    (if (== Track (`self.WolfDirection`))
      (`self.Catch`)
      (else
        (`self.Fail` Track)))))

(event `Pause`
  (bind _asbp_console_pawn (cast `/Game/Blueprints/BP_Console_Pawn` (`GameplayStatics.GetPlayerPawn` 0) :!pure true))
  ;[1 1 1] Pause
  (`/Engine/EditorBlueprintResources/StandardMacros.FlipFlop`
    (:`A`
      (set `Actor.CustomTimeDilation` 0.0 _asbp_console_pawn))
    (:`B`
      (set `Actor.CustomTimeDilation` 1.0 _asbp_console_pawn))))

(event `Fail`
  (params (Track :type Integer))
  (bind _asbp_console_pawn (cast `/Game/Blueprints/BP_Console_Pawn` (`GameplayStatics.GetPlayerPawn` 0) :!pure true))
  ;[1 1 1] Fail / Catch
  (set `self.isFell` true)
  (`self.FailIncrement`)
  (`/Game/Blueprints/BP_Console_Pawn.EggsTurnOff` _asbp_console_pawn)
  (`/Game/Blueprints/BP_Console_Pawn.FellRender` _asbp_console_pawn Track)
  (`/Game/Blueprints/BP_Console_Pawn.FailRender` _asbp_console_pawn)
  (if (>= (`self.Fails`) 6)
    (`self.GameOver`)
    (`self.SaveScore`)))

(event `Catch`
  ;[1 1 1] Fail / Catch
  (`self.ScoreIncrement`)
  (`self.CheckForBonus`)
  (`/Game/Blueprints/BP_Console_Pawn.ScoreRender` (cast `/Game/Blueprints/BP_Console_Pawn` (`GameplayStatics.GetPlayerPawn` 0) :!pure true)))

(event `GameOver`
  ;[1 1 1] Game Over
  (set `self.isGameStarted` false)
  (`KismetSystemLibrary.Delay` 3.5)
  (`/Game/Blueprints/BP_Console_Pawn.GOSound` (cast `/Game/Blueprints/BP_Console_Pawn` (`GameplayStatics.GetPlayerPawn` 0) :!pure true)))

(event `SaveScore`
  (bind _returnvalue (`GameplayStatics.DoesSaveGameExist` "Highscore"))
  (if _returnvalue
    (bind _returnvalue_2 (`GameplayStatics.LoadGameFromSlot` "Highscore"))
    (bind _output_get (set `self.SaveGameRef` _returnvalue_2))
    (bind _asbp_highscore_save (cast `/Game/Blueprints/BP_Highscore_Save` _output_get))
    (`KismetArrayLibrary.Array_Add` (`/Game/Blueprints/BP_Highscore_Save.Score` _asbp_highscore_save) (`self.Score`))
    (`KismetArrayLibrary.Array_Add` (`/Game/Blueprints/BP_Highscore_Save.PlayerNames` _asbp_highscore_save) (`self.PlayerName`))
    (else
      (bind _returnvalue_3 (`GameplayStatics.CreateSaveGameObject` "/Game/Blueprints/BP_Highscore_Save.BP_Highscore_Save_C"))
      (bind _output_get_2 (set `self.SaveGameRef` _returnvalue_3))
      (bind _asbp_highscore_save_2 (cast `/Game/Blueprints/BP_Highscore_Save` _output_get_2))
      (`KismetArrayLibrary.Array_Add` (`/Game/Blueprints/BP_Highscore_Save.Score` _asbp_highscore_save_2) (`self.Score`))
      (`KismetArrayLibrary.Array_Add` (`/Game/Blueprints/BP_Highscore_Save.PlayerNames` _asbp_highscore_save_2) (`self.PlayerName`))))
  (`GameplayStatics.SaveGameToSlot` (`self.SaveGameRef`) "Highscore")
  (`KismetSystemLibrary.PrintString` "saved"))

(fn `CheckForBonus`
  (bind _score (`self.Score`))
  (if (or (== _score 200) (== _score 500))
    (bind _output_get (set `self.Fails` (- (`self.Fails`) 2)))
    (if (< _output_get 0)
      (set `self.Fails` 0)
      (`/Game/Blueprints/BP_Console_Pawn.FailRender` (cast `/Game/Blueprints/BP_Console_Pawn` (`GameplayStatics.GetPlayerPawn` 0) :!pure true))))
  (return))

(fn `FailIncrement`
  (bind _fails (`self.Fails`))
  (if (`self.isRabbit`)
    (set `self.Fails` (+ _fails 1))
    (else
      (set `self.Fails` (+ _fails 2))))
  (return))

(fn `GetTrack`
  (returns (Track :type Integer))
  (locals (AllTracks :type "Array of Integer") (ExceptLeftBottom :type "Array of Integer") (ExeptRightBottom :type "Array of Integer") (ExeptLeftTop :type "Array of Integer") (ExeptRightTop :type "Array of Integer") (AvailableTracks :type "Array of Integer"))
  (bind _exeptrightbottom (`local.ExeptRightBottom`))
  (bind _exeptlefttop (`local.ExeptLeftTop`))
  (if (`self.GameMode`)
    (set `local.AvailableTracks` (`local.AllTracks`))
    (else
      (set `local.AvailableTracks` (select `int` (`self.Fails`) :`0` (`local.ExceptLeftBottom`) :`1` _exeptrightbottom :`2` _exeptrightbottom :`3` _exeptlefttop :`4` _exeptlefttop :`5` (`local.ExeptRightTop`)))))
  (if (== (`self.LastUsedTrack`) -1)
    (set `self.LastUsedTrack` (`KismetArrayLibrary.Array_Random` (`local.AvailableTracks`)))
    (else
      (`KismetArrayLibrary.Array_RemoveItem` (`local.AvailableTracks`) (`self.LastUsedTrack`))
      (set `self.LastUsedTrack` (`KismetArrayLibrary.Array_Random` (`local.AvailableTracks`)))))
  (return (`self.LastUsedTrack`)))

(fn `ScoreIncrement`
  (set `self.Score` (+ (`self.Score`) 1))
  (`AudioComponent.Play` (`/Game/Blueprints/BP_Console_Pawn.Catch` (cast `/Game/Blueprints/BP_Console_Pawn` (`GameplayStatics.GetPlayerPawn` 0) :!pure true)) 0.0))

(fn `Spawn`
  (bind _track (`self.GetTrack`))
  (`/Game/Blueprints/BP_Console_Pawn.EggRender` (cast `/Game/Blueprints/BP_Console_Pawn` (`GameplayStatics.GetPlayerPawn` 0) :!pure true) _track))

(fn `UpdateIntervals`
  (bind _score (`self.Score`))
  (bind _mineggtick (`self.MinEggTick`))
  (bind _mineggspawninterval (`self.MinEggSpawnInterval`))
  (if (`self.GameMode`)
    (if (not (`self.isAdjustedForGameB`))
      (set `self.EggTick` (* (`self.EggTick`) 0.75))
      (set `self.EggSpawnInterval` (* (`self.EggSpawnInterval`) 0.75))
      (set `self.isAdjustedForGameB` true)))
  (if (or (== _score 200) (== _score 500))
    (set `self.EggTick` (* (`self.EggTick`) 1.5))
    (set `self.EggSpawnInterval` (* (`self.EggSpawnInterval`) 1.5))
    (elif (or (== _score 5) (== _score 25) (== _score 50) (== _score 100) (== _score 150))
      (set `self.EggTick` (* (`self.EggTick`) 0.95))
      (set `self.EggSpawnInterval` (* (`self.EggSpawnInterval`) 0.9))
      (else
        (set `self.EggTick` (* (`self.EggTick`) 0.995))
        (set `self.EggSpawnInterval` (* (`self.EggSpawnInterval`) 0.9985)))))
  (`|ExecutionSequence`
    (:`then_0`
      (if (not (>= (`self.EggTick`) _mineggtick))
        (set `self.EggTick` _mineggtick)))
    (:`then_1`
      (if (not (>= (`self.EggSpawnInterval`) _mineggspawninterval))
        (set `self.EggSpawnInterval` _mineggspawninterval))))
  (return))

(fn `UserConstructionScript`)